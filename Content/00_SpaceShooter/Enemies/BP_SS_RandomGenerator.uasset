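; BP_SS_RandomGenerator is the space shooter's enemy spawner, creating a random enemy on a looping timer.
; SpawnEnemy picks a random SpawnerPoint-tagged component for location and a class from a random index bounded by the game mode's Level, clamped to MaxNumEnemies.
; Each enemy's destroy event decrements SpawnTime, though the running timer keeps the interval set at BeginPlay.
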(event Custom|Spawn
  (bind _enemyspawned (CallFunction|SpawnEnemy))
  (bind _asbp_ss_enemy_base (Utilities|Casting|CastToBP_SS_EnemyBase _enemyspawned))
  (EventDispatchers|BindEventtoOnEnemyDestroy _asbp_ss_enemy_base (delegate Custom|EnemyDestroyed)))

(event Custom|EnemyDestroyed
  (Variables|Default|SetSpawnTime (- (Variables|Default|GetSpawnTime) 1.0)))

(event EventBeginPlay
  (Utilities|Time|SetTimerbyEvent (delegate Custom|Spawn) (Variables|Default|GetSpawnTime) true)
  (bind _asbp_ss_game_mode (Utilities|Casting|CastToBP_SS_GameMode (Game|GetGameMode)))
  (Variables|Default|SetSS%20Game%20Mode _asbp_ss_game_mode))

(event Collision|EventActorBeginOverlap
  (params (OtherActor :type Actor%20Object%20Reference)))

(event EventTick
  (params (DeltaSeconds :type Float%20%28single-precision%29)))

(fn ConstructionScript)

(fn SpawnEnemy
  (bind _returnvalue (Actor|GetComponentsbyTag "/Script/Engine.SceneComponent" "SpawnerPoint"))
  (bind _class (CallFunction|GetClass2Spawn (Math|Random|RandomInteger (Variables|/Game/00_SpaceShooter/BP_SS_GameMode.BP_SS_GameMode_C|GetLevel (Variables|Default|GetSS%20Game%20Mode)))))
  (bind _returnvalue_2 (Game|SpawnActorfromClass _class (Transformation|GetWorldTransform (Utilities|Array|Get(acopy) _returnvalue (Math|Random|RandomInteger (Utilities|Array|Length _returnvalue)))) "Undefined" "MultiplyWithRoot" 0 0))
  (bind _asbp_ss_enemy_base (Utilities|Casting|CastToBP_SS_EnemyBase _returnvalue_2))
  (return _asbp_ss_enemy_base))

(fn GetClass2Spawn
  (params (Type :type Integer))
  (return (Utilities|Select :Index (Math|Integer|Clamp(Integer) Type 0 (- (Variables|Default|GetMaxNumEnemies) 1)) :Option%200 "/Game/00_SpaceShooter/Enemies/BP_SS_EnemyBase.BP_SS_EnemyBase_C" :Option%201 "/Game/00_SpaceShooter/Enemies/BP_SS_EnemyH.BP_SS_EnemyH_C")))