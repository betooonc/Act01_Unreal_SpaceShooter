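; BP_SS_EnemyAmmo is an enemy projectile for the space shooter.
; Each tick it moves along its forward vector at a Speed-scaled rate, without sweeping.
; On overlap with a Pawn not tagged Enemy, it spawns an emitter at its location, then destroys itself after a short delay.
; The graph applies no damage itself.
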(event EventBeginPlay)

(event Collision|EventActorBeginOverlap
  (params (OtherActor :type Actor%20Object%20Reference))
  (if (not (Utilities|Array|ContainsItem (Variables|/Script/Engine.Actor|GetTags OtherActor) "Enemy"))
    (Utilities|Casting|CastToPawn OtherActor)
    (Effects|SpawnEmitteratLocation 0 (Transformation|GetActorLocation))
    (Utilities|FlowControl|Delay 0.2)
    (Actor|DestroyActor)))

(event EventTick
  (params (DeltaSeconds :type Float%20%28single-precision%29))
  ;[1 1 1] Move the ammo forward
  (Transformation|SetActorLocation (+ (Transformation|GetActorLocation) (* (Transformation|GetActorForwardVector) (* DeltaSeconds (Variables|Default|GetSpeed)))) false false))

(fn ConstructionScript)