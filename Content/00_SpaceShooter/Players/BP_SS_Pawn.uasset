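; Player pawn for the space shooter that moves with Enhanced Input, with firing currently a placeholder debug print.
; BeginPlay adds the player mapping context to the local player's input subsystem.
; Movement input is stored while triggered and zeroed on cancel or completion.
; Tick applies that saved vector along the actor's right and forward axes, scaled by speed and delta time, setting location without sweep, so movement ignores collision.
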(event Input|EnhancedActionEvents|EnhancedInputActionIA_SS_PlayerFire
  (params (ActionValue :type Boolean) (ElapsedSeconds :type Float%20%28double-precision%29) (TriggeredSeconds :type Float%20%28double-precision%29) (InputAction :type Input%20Action%20Object%20Reference :default "/Game/00_SpaceShooter/Input/IA_SS_PlayerFire.IA_SS_PlayerFire"))
  (Development|PrintString "Fire!"))

(event Input|EnhancedActionEvents|EnhancedInputActionIA_SS_PlayerMovement
  (params (ActionValue :type Vector%202D%20Structure) (ElapsedSeconds :type Float%20%28double-precision%29) (TriggeredSeconds :type Float%20%28double-precision%29) (InputAction :type Input%20Action%20Object%20Reference :default "/Game/00_SpaceShooter/Input/IA_SS_PlayerMovement.IA_SS_PlayerMovement"))
  (:Triggered
    (Variables|Default|SetInputMovement_Saved ActionValue))
  (:Canceled
    (Variables|Default|SetInputMovement_Saved "" :!label _label))
  (:Completed
    (goto _label)))

(event EventBeginPlay
  ;[1 1 1] Setup New Enhanced Input
  (bind _asplayer_controller (Utilities|Casting|CastToPlayerController (Pawn|GetController)))
  (Utilities|IsValid (PlayerController|LocalPlayerSubsystems|GetEnhancedInputLocalPlayerSubsystem _asplayer_controller)
    (:Is%20Valid
      (Input|AddMappingContext (PlayerController|LocalPlayerSubsystems|GetEnhancedInputLocalPlayerSubsystem _asplayer_controller) "/Game/00_SpaceShooter/Input/IMC_SS_Player.IMC_SS_Player" 0 "(bIgnoreAllPressedKeysUntilRelease=True,bForceImmediately=False,bNotifyUserSettings=False)"))))

(event Collision|EventActorBeginOverlap
  (params (OtherActor :type Actor%20Object%20Reference)))

(event EventTick
  (params (DeltaSeconds :type Float%20%28single-precision%29))
  (bind _speed (Variables|Default|GetSpeed))
  (bind _inputmovement_saved (Variables|Default|GetInputMovement_Saved))
  (bind _returnvalue (* DeltaSeconds _speed))
  ;[1 1 1] Update Movement
  (Transformation|SetActorLocation (+ (+ (* (Transformation|GetActorRightVector) (* _returnvalue (.x _inputmovement_saved))) (* (* _returnvalue (.y _inputmovement_saved)) (Transformation|GetActorForwardVector))) (Transformation|GetActorLocation)) false false))

(fn ConstructionScript)